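; Holograph generator actor that computes point sets for a Hopalong-style attractor, regenerated on a looping timer.
; Each pass randomizes the shared equation parameters, seeds each orbit's start point from a random stream and iterates it into one flat Points array, offset by running bounds.
; It also builds a small random-hue palette for cycled lookup.
; The first pass notifies HolographController; later passes only print a debug message.
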(event Custom|GenerateHolograph
  ;[1 1 1] Initialize orbits and generate points for all of them
  (CallFunction|RandomizeParams)
  (for _index (range 0 (- (Variables|Default|GetNUM_ORBITS) 1))
    (CallFunction|GenerateOrbit _index))
  (CallFunction|GenerateColorPalette)
  ;[1 1 1] Notify listeners that points were (re)generated
  (if (Variables|Default|GetHasGenerated)
    (Development|PrintString "Orbit Generated" true true "(R=1.000000,G=0.810141,B=0.000000,A=1.000000)")
    (else
      (Variables|Default|SetHasGenerated true)
      (Class|BPIHolograph|InitialPointsGenerated(Message) (Variables|Default|GetHolographController)))))

(event EventBeginPlay
  (Utilities|Time|SetTimerbyFunctionName 0 "GenerateHolograph" (Variables|Default|Getinterval) true)
  ;[1 1 1] Initialize orbits and generate points for all of them
  (CallFunction|InitializeOrbits)
  (CallFunction|RandomizeParams)
  (for _index (range 0 (- (Variables|Default|GetNUM_ORBITS) 1))
    (CallFunction|GenerateOrbit _index))
  (CallFunction|GenerateColorPalette)
  ;[1 1 1] Notify listeners that points were (re)generated
  (if (Variables|Default|GetHasGenerated)
    (Development|PrintString "Orbit Generated" true true "(R=1.000000,G=0.810141,B=0.000000,A=1.000000)")
    (else
      (Variables|Default|SetHasGenerated true)
      (Class|BPIHolograph|InitialPointsGenerated(Message) (Variables|Default|GetHolographController)))))

(event Collision|EventActorBeginOverlap
  (params (OtherActor :type Actor%20Object%20Reference)))

(event EventTick
  (params (DeltaSeconds :type Float%20%28single-precision%29)))

(fn ConstructionScript)

(fn InitializeOrbits
  (bind _points (Variables|Default|Getpoints))
  (Utilities|Array|Clear _points)
  (for _index (range 0 (- (* (Variables|Default|GetnumPointsOrbit) (Variables|Default|GetNUM_ORBITS)) 1))
    (Utilities|Array|Add :TargetArray _points))
  (return))

(fn RandomizeParams
  (bind _orbit_max (Variables|Default|GetORBIT_MAX))
  (bind _returnvalue (Math|Random|RandomFloatinRange 0.0 _orbit_max))
  (Variables|Default|Seta (* _returnvalue (- (Variables|Default|GetA_MAX) (Variables|Default|GetA_MIN))))
  (Variables|Default|Setb (* _returnvalue (- (Variables|Default|GetB_MAX) (Variables|Default|GetB_MIN))))
  (Variables|Default|Setc (* _returnvalue (- (Variables|Default|GetC_MAX) (Variables|Default|GetC_MIN))))
  (Variables|Default|Setd (* _returnvalue (- (Variables|Default|GetD_MAX) (Variables|Default|GetD_MIN))))
  (Variables|Default|Sete (* _returnvalue (- (Variables|Default|GetE_MAX) (Variables|Default|GetE_MIN))))
  (return))

(fn InitializeOrbitParams
  (params (idx :type Integer))
  (bind _randomstream (Variables|Default|GetrandomStream))
  (bind _returnvalue (Math|Random|RandomFloatfromStream _randomstream))
  (bind _returnvalue_2 (- 0.5 _returnvalue))
  (bind _returnvalue_3 (* idx 0.005 _returnvalue_2))
  (Variables|Default|Setx _returnvalue_3)
  (Variables|Default|Sety _returnvalue_3)
  (Variables|Default|SetxMin 0.0)
  (Variables|Default|SetxMax 0.0)
  (Variables|Default|SetyMin 0.0)
  (Variables|Default|SetyMax 0.0)
  (return))

(fn CalculateOrbit
  (params (a :type Float%20%28double-precision%29) (b :type Float%20%28double-precision%29) (c :type Float%20%28double-precision%29) (d :type Float%20%28double-precision%29) (e :type Float%20%28double-precision%29))
  (Variables|Default|Setz (+ d (Math|Float|Sqrt (Math|Float|Absolute(Float) (- (* b (Variables|Default|Getx)) c)))))
  (if (> (Variables|Default|Getx) 0.0)
    (Variables|Default|Setx1 (- (Variables|Default|Gety) (Variables|Default|Getz))))
  (if (== (Variables|Default|Getx) 0.0)
    (Variables|Default|Setx1 (Variables|Default|Gety)))
  (if (< (Variables|Default|Getx) 0.0)
    (Variables|Default|Setx1 (+ (Variables|Default|Gety) (Variables|Default|Getz))))
  (Variables|Default|Sety (- a (Variables|Default|Getx)))
  (bind _output_get (Variables|Default|Setx (+ (Variables|Default|Getx1) e)))
  (if (< _output_get (Variables|Default|GetxMin))
    (Variables|Default|SetxMin (Variables|Default|Getx)))
  (if (> (Variables|Default|Getx) (Variables|Default|GetxMax))
    (Variables|Default|SetxMax (Variables|Default|Getx)))
  (if (< (Variables|Default|Gety) (Variables|Default|GetyMin))
    (Variables|Default|SetyMin (Variables|Default|Gety)))
  (if (> (Variables|Default|Gety) (Variables|Default|GetyMax))
    (Variables|Default|SetyMax (Variables|Default|Gety)))
  (return (Variables|Default|Gety) (Variables|Default|Getx) (Variables|Default|GetxMin) (Variables|Default|GetxMax) (Variables|Default|GetyMin) (Variables|Default|GetyMax)))

(fn GenerateOrbit
  (params (idx :type Integer))
  (bind _numpointsorbit (Variables|Default|GetnumPointsOrbit))
  (CallFunction|InitializeOrbitParams idx)
  (for _index (range 0 (- _numpointsorbit 1))
    (bind (_y _x _xmin _xmax _ymin _ymax) (CallFunction|CalculateOrbit (Variables|Default|Geta) (Variables|Default|Getb) (Variables|Default|Getc) (Variables|Default|Getd) (Variables|Default|Gete)))
    (Utilities|Array|SetArrayElem (Variables|Default|Getpoints) (+ _index (* idx _numpointsorbit)) (Math|Vector|MakeVector (Utilities|Operators|Subtract _x _xmin (/ (- _xmax _xmin) 2.0)) (Utilities|Operators|Subtract _y _ymin (/ (- _ymax _ymin) 2.0)) 0.0))))

(fn GenerateColorPalette
  (bind _color (Variables|Default|Getcolor))
  (bind _output_get (Variables|Default|SetcolorCount (Math|Random|RandomIntegerinRangefromStream 2 5 (Variables|Default|GetrandomStream))))
  (Utilities|Array|Clear (Variables|Default|Getcolors))
  (Variables|Default|SetcolorIdx 0)
  (bind _index (Utilities|FlowControl|ForLoopwithBreak 0 (- _output_get 1))
    (:LoopBody
      (Class|KismetMathLibrary|LinearColorSetRandomHue _color)
      (Utilities|Array|SetArrayElem (Variables|Default|Getcolors) _index _color true))
    (:Completed
      (return))))

(fn GetNextColor
  (if (< (Variables|Default|GetcolorIdx) (Variables|Default|GetcolorCount))
    (Variables|Default|Setcolor (Utilities|Array|Get(acopy) (Variables|Default|Getcolors) (Variables|Default|GetcolorIdx)))
    (Variables|Default|SetcolorIdx (+ (Variables|Default|GetcolorIdx) 1))
    (else
      (Variables|Default|SetcolorIdx 0)
      (Variables|Default|Setcolor (Utilities|Array|Get(acopy) (Variables|Default|Getcolors) (Variables|Default|GetcolorIdx)))))
  (return (Variables|Default|Getcolor)))

(fn InitialPointsGenerated)

(fn PointsRegenerated
  (return))
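; BP_Holograph is a holograph actor that scrolls along negative world X in a looping band and displays points through a Niagara system.
; BeginPlay derives the clipping end from BP_HolographController's spacing and count, then pushes BP_LatestHolograph's points into the Niagara "Points" array.
; Tick moves the actor by Speed, teleporting it to the opposite end once past the clipping end and refreshing the points from BP_LatestHolograph.
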(event EventBeginPlay
  (bind _returnvalue (Actor|GetActorOfClass "/Game/Blueprints/BP_LatestHolograph.BP_LatestHolograph_C"))
  ;[1 1 1] Calculate and set holograph bounds
  (bind _returnvalue_2 (Actor|GetActorOfClass "/Game/Blueprints/BP_HolographController.BP_HolographController_C"))
  (Variables|Default|SetclippingEnd (* (Variables|/Game/Blueprints/BP_HolographController.BP_HolographController_C|GetspaceBetween _returnvalue_2) (Variables|/Game/Blueprints/BP_HolographController.BP_HolographController_C|Getcount _returnvalue_2) -1))
  (Class|NiagaraDataInterfaceArrayFunctionLibrary|SetNiagaraArrayPosition (Variables|Default|GetNS_Holograph) "Points" (Variables|/Game/Blueprints/BP_LatestHolograph.BP_LatestHolograph_C|Getpoints _returnvalue)))

(event EventTick
  (params (DeltaSeconds :type Float%20%28single-precision%29))
  (bind _returnvalue (Transformation|GetActorTransform))
  (bind _returnvalue_2 (Transformation|GetActorTransform))
  (bind _clippingend (Variables|Default|GetclippingEnd))
  ;[1 1 1] Transform self over time and move to the beginning when we hit the end of the clipping plane
  (if (< (.x (.location _returnvalue)) _clippingend)
    (Transformation|SetActorTransform (Math|Transform|MakeTransform (Math|Vector|MakeVector (* _clippingend -1.0) (.y (.location _returnvalue_2)) (.z (.location _returnvalue_2))) (.rotation _returnvalue_2) (.scale _returnvalue_2)) false true)
    (Development|PrintString "Reached end of clipping plane and reset")
    (Class|NiagaraDataInterfaceArrayFunctionLibrary|SetNiagaraArrayPosition (Variables|Default|GetNS_Holograph) "Points" (Variables|/Game/Blueprints/BP_LatestHolograph.BP_LatestHolograph_C|Getpoints (stale EventBeginPlay _returnvalue)))
    (else
      (Transformation|SetActorTransform (Math|Transform|MakeTransform (Math|Vector|MakeVector (- (.x (.location _returnvalue)) (* DeltaSeconds (Variables|Default|GetSpeed))) (.y (.location _returnvalue)) (.z (.location _returnvalue))) (.rotation _returnvalue) (.scale _returnvalue)) false true))))

(fn ConstructionScript)

(fn InitialPointsGenerated
  (return))